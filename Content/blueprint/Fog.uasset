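; Fog is a hazard actor that deals periodic damage to player characters (主角) standing inside its sphere volume.
; Sphere overlap events cast to 主角 and add or remove the character from the Enemy array.
; A Damage loop started on BeginPlay applies a fixed damage to every array entry, waits on a one-second Delay, then repeats for the actor's lifetime.
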(event OnComponentBeginOverlap(Sphere)
  (params (OverlappedComponent :type Primitive%20Component%20Object%20Reference) (OtherActor :type Actor%20Object%20Reference) (OtherComp :type Primitive%20Component%20Object%20Reference) (OtherBodyIndex :type Integer) (bFromSweep :type Boolean) (SweepResult :type Hit%20Result%20Structure%20%28by%20ref%29))
  (bind _as主角 (Utilities|Casting|CastTo主角 OtherActor))
  (Utilities|Array|Add (Variables|Default|GetEnemy) _as主角))

(event OnComponentEndOverlap(Sphere)
  (params (OverlappedComponent :type Primitive%20Component%20Object%20Reference) (OtherActor :type Actor%20Object%20Reference) (OtherComp :type Primitive%20Component%20Object%20Reference) (OtherBodyIndex :type Integer))
  (bind _as主角 (Utilities|Casting|CastTo主角 OtherActor))
  (Utilities|Array|RemoveItem (Variables|Default|GetEnemy) _as主角))

(event Custom|Damage
  (for _array_element (Variables|Default|GetEnemy) :!label _label
    (Game|Damage|ApplyDamage _array_element 1e+01 0 0))
  (Utilities|FlowControl|Delay 1.0)
  (goto _label))

(event EventBeginPlay
  (CallFunction|Damage))

(event Collision|EventActorBeginOverlap
  (params (OtherActor :type Actor%20Object%20Reference)))

(event EventTick
  (params (DeltaSeconds :type Float%20%28single-precision%29)))

(fn ConstructionScript)