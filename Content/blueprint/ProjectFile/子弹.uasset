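; Bullet projectile that damages enemies and explodes on hit or when it slows down.
; On BeginPlay, its physics Sphere launches along the actor's forward vector at Speed.
; Sphere1 overlap with an Enemy applies BaseDamage, spawns an Explosion and destroys the bullet after a short delay.
; Tick watches the Sphere's velocity and, once it falls to a low threshold, triggers a one-time explosion and the same delayed destruction.
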(event OnComponentBeginOverlap(Sphere1)
  (params (OverlappedComponent :type Primitive%20Component%20Object%20Reference) (OtherActor :type Actor%20Object%20Reference) (OtherComp :type Primitive%20Component%20Object%20Reference) (OtherBodyIndex :type Integer) (bFromSweep :type Boolean) (SweepResult :type Hit%20Result%20Structure%20%28by%20ref%29))
  (bind _asenemy (Utilities|Casting|CastToEnemy OtherActor))
  (Game|Damage|ApplyDamage _asenemy (Variables|Default|GetBase%20Damage) 0 0)
  (Game|SpawnActorfromClass "/Game/blueprint/ProjectFile/Explosion.Explosion_C" (Transformation|GetActorTransform) "AlwaysSpawn" 0 0)
  (Utilities|FlowControl|Delay 1.0)
  (Actor|DestroyActor))

(event EventBeginPlay
  (Physics|SetPhysicsLinearVelocity (Variables|Default|GetSphere) (* (Math|Vector|GetForwardVector (Transformation|GetActorRotation)) (Variables|Default|Getspeed)) false "None"))

(event Collision|EventActorBeginOverlap
  (params (OtherActor :type Actor%20Object%20Reference)))

(event EventTick
  (params (DeltaSeconds :type Float%20%28single-precision%29))
  (bind _returnvalue (Physics|GetPhysicsLinearVelocity (Variables|Default|GetSphere) "None"))
  (if (<= (Math|Vector|VectorLength _returnvalue) 5e+02)
    (Utilities|FlowControl|DoOnce false
      (:Completed
        (Game|SpawnActorfromClass "/Game/blueprint/ProjectFile/Explosion.Explosion_C" (Transformation|GetWorldTransform (Variables|Default|GetSphere)) "AlwaysSpawn" 0 0)
        (Utilities|FlowControl|Delay 1.0)
        (Actor|DestroyActor)))))

(fn ConstructionScript)