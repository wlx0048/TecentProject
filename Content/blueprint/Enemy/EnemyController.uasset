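; Enemy AI controller that runs the BT_Enemy1 behavior tree on possession and feeds player sightings into its Blackboard.
; When AI perception senses an actor tagged Player, a one-shot timer delays detection, and any other perception update cancels it.
; When the timer fires, it sets HasLineOfSight and stores the sensed actor as EnemyActor, with no path here that resets them.
; A separate SetReceived event sets a variable-named Blackboard bool to true.
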(event OnTargetPerceptionUpdated(AIPerception)
  (params (Actor :type Actor%20Object%20Reference) (Stimulus :type AI%20Stimulus%20Structure))
  (if (and (.bSuccessfullySensed (Utilities|Struct|BreakAIStimulus Stimulus)) (Actor|ActorHasTag Actor "Player"))
    (bind _returnvalue (Utilities|Time|SetTimerbyEvent (delegate Custom|StartEnemy) (Variables|Default|GetTime)))
    (Variables|Default|SetEnemyTimer _returnvalue)
    (else
      (Utilities|Time|ClearandInvalidateTimerbyHandle (Variables|Default|GetEnemyTimer)))))

(event Custom|StartEnemy
  (bind _blackboard (Variables|Default|GetBlackboard))
  (AI|Components|Blackboard|SetValueasBool _blackboard (Variables|Default|GetHasLineOfSight) true)
  (AI|Components|Blackboard|SetValueasObject _blackboard (Variables|Default|GetEnemyActor) (stale OnTargetPerceptionUpdated(AIPerception) Actor)))

(event Custom|SetReceived
  (AI|Components|Blackboard|SetValueasBool (Variables|Default|GetBlackboard) (Variables|Default|GetKey%20Name) true))

(event EventBeginPlay)

(event EventTick
  (params (DeltaSeconds :type Float%20%28single-precision%29)))

(event EventPossess
  (params (PossessedPawn :type Pawn%20Object%20Reference))
  (AI|RunBehaviorTree "/Game/blueprint/Enemy/BehaviorTree/BT_Enemy1.BT_Enemy1"))

(fn ConstructionScript)