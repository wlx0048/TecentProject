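; Weapon pickup actor that the player character (主角) can collect while standing inside its sphere trigger.
; Sphere overlaps open and close a gate and, until picked up, tell the player controller to create or destroy the weapon widget.
; When the 拿起武器！ (pick up weapon) event passes the open gate, it sets IsPick, has the character spawn a gun of this actor's class, then destroys itself.
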(event OnComponentBeginOverlap(Sphere)
  (params (OverlappedComponent :type Primitive%20Component%20Object%20Reference) (OtherActor :type Actor%20Object%20Reference) (OtherComp :type Primitive%20Component%20Object%20Reference) (OtherBodyIndex :type Integer) (bFromSweep :type Boolean) (SweepResult :type Hit%20Result%20Structure%20%28by%20ref%29))
  (Utilities|FlowControl|Sequence
    (:then_0
      (bind _as主角 (Utilities|Casting|CastTo主角 OtherActor))
      (Utilities|FlowControl|Gate true) ; enters at Open
    )
    (:then_1
      (bind _as主角_2 (Utilities|Casting|CastTo主角 OtherActor))
      (if (not (Variables|Default|GetisPick))
        (bind _as1playercontroller (Utilities|Casting|CastTo1playercontroller (Pawn|GetController _as主角_2)))
        (Default|CreateWeaponWidgt _as1playercontroller self)))))

(event OnComponentEndOverlap(Sphere)
  (params (OverlappedComponent :type Primitive%20Component%20Object%20Reference) (OtherActor :type Actor%20Object%20Reference) (OtherComp :type Primitive%20Component%20Object%20Reference) (OtherBodyIndex :type Integer))
  (Utilities|FlowControl|Sequence
    (:then_0
      (Utilities|Casting|CastTo主角 OtherActor)
      (Utilities|FlowControl|Gate true) ; enters at Close
    )
    (:then_1
      (bind _as主角 (Utilities|Casting|CastTo主角 OtherActor))
      (if (not (Variables|Default|GetisPick))
        (bind _as1playercontroller (Utilities|Casting|CastTo1playercontroller (Pawn|GetController _as主角)))
        (Default|DestroyWeaponWidgt _as1playercontroller)))))

(event Custom|拿起武器！
  (Utilities|FlowControl|Gate true
    (:Exit
      (Variables|Default|SetisPick true)
      (Default|SpawnGun (stale OnComponentBeginOverlap(Sphere) _as主角) (Utilities|GetClass self))
      (Actor|DestroyActor))))

(event EventBeginPlay)

(event Collision|EventActorBeginOverlap
  (params (OtherActor :type Actor%20Object%20Reference)))

(event EventTick
  (params (DeltaSeconds :type Float%20%28single-precision%29)))

(fn ConstructionScript)