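; Player controller that manages the local player's UI and can reset the player state's health to its maximum.
; On client login it adds HUD, aim and name-agnostic player input widgets, switching input to UI-only focused on the latter.
; Events add and remove a weapon pick widget for a given weapon.
; Tick polls the game state's timer and shows the score widget once it reaches zero.
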(event Custom|ClientLoginOn
  (CallFunction|CreateWidgt))

(event Custom|CreateWeaponWidgt
  (params (NewParam :type 1%20Weapon%20Object%20Reference))
  (bind _returnvalue (UserInterface|CreateWidget "/Game/blueprint/widget/WeaponPick.WeaponPick_C" self NewParam))
  (UserInterface|Viewport|AddtoViewport _returnvalue 0))

(event Custom|DestroyWeaponWidgt
  (Widget|RemovefromParent (stale Custom|CreateWeaponWidgt _returnvalue)))

(event Custom|ResetHealth
  (bind _asmy_player_state (Utilities|Casting|CastToMyPlayerState (Variables|GetPlayerState)))
  (Variables|/Game/blueprint/myplayerstate.MyPlayerState_C|SetHealth _asmy_player_state (Variables|/Game/blueprint/myplayerstate.MyPlayerState_C|GetMaxHealth _asmy_player_state)))

(event Custom|CreateScore
  (bind _returnvalue (UserInterface|CreateWidget "/Game/blueprint/widget/Score.Score_C"))
  (UserInterface|Viewport|AddtoViewport _returnvalue 0))

(event EventBeginPlay
  (Development|PrintString (Utilities|GetDisplayName (Pawn|GetControlledPawn))))

(event EventTick
  (params (DeltaSeconds :type Float%20%28single-precision%29))
  (bind _asmy_game_state (Utilities|Casting|CastToMyGameState (Game|GetGameState)))
  (if (== (Variables|/Game/blueprint/MyGameState.MyGameState_C|GetTime _asmy_game_state) 0.0)
    (Utilities|FlowControl|DoOnce false
      (:Completed
        (CallFunction|CreateScore)))))

(fn ConstructionScript)

(fn CreateWidgt
  (if (Pawn|IsLocalPlayerController)
    (bind _returnvalue (UserInterface|CreateWidget "/Game/blueprint/widget/MyHUD.MyHUD_C" self))
    (bind _output_get (Variables|Default|SetMainHUD _returnvalue))
    (UserInterface|Viewport|AddtoViewport _output_get 0)
    (bind _returnvalue_2 (UserInterface|CreateWidget "/Game/blueprint/widget/Aim.Aim_C" self))
    (bind _output_get_2 (Variables|Default|SetAimingHUD _returnvalue_2))
    (UserInterface|Viewport|AddtoViewport _output_get_2 0)
    (bind _returnvalue_3 (UserInterface|CreateWidget "/Game/blueprint/widget/InputPlayer.InputPlayer_C" self))
    (UserInterface|Viewport|AddtoViewport _returnvalue_3 10)
    (Input|SetInputModeUIOnly self _returnvalue_3 "DoNotLock")))