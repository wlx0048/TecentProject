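; AI controller for an enemy that runs the BT_Enemy3 behavior tree when it possesses its pawn.
; On the first tick, a DoOnce finds the protagonist actor (主角) by class and stores it in the EnemyActor blackboard key as the enemy's target.
; A SetReceived event sets a boolean blackboard key to true.
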(event Custom|SetReceived
  (AI|Components|Blackboard|SetValueasBool (Variables|Default|GetBlackboard) (Variables|Default|GetKey%20Name) true))

(event EventBeginPlay)

(event EventTick
  (params (DeltaSeconds :type Float%20%28single-precision%29))
  (Utilities|FlowControl|DoOnce false
    (:Completed
      (bind _returnvalue (Actor|GetActorOfClass "/Game/blueprint/主角.主角_C"))
      (AI|Components|Blackboard|SetValueasObject (Variables|Default|GetBlackboard) (Variables|Default|GetEnemyActor) _returnvalue))))

(event EventPossess
  (params (PossessedPawn :type Pawn%20Object%20Reference))
  (AI|RunBehaviorTree "/Game/blueprint/Enemy/BehaviorTree/BT_Enemy3.BT_Enemy3"))

(fn ConstructionScript)