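; Enemy actor with health, a floating health bar widget, and a random item drop on death.
; The Health widget is initialized on begin play, turned toward the player camera every tick, and updated on damage.
; At zero health it ragdolls, is destroyed after a short delay, and increments the instigator's score.
; A drop roll made at spawn decides between a Buff, an AKM, or nothing.
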(event Custom|Die
  (params (Instigater :type Controller%20Object%20Reference))
  (bind _returnvalue (Transformation|GetActorTransform))
  (Pawn|Components|CharacterMovement|DisableMovement (Variables|Character|GetCharacterMovement))
  (Physics|SetSimulatePhysics (Variables|Character|GetMesh) true)
  (Utilities|FlowControl|Delay 1.0)
  (Actor|DestroyActor)
  (bind _asmy_player_state (Utilities|Casting|CastToMyPlayerState (Variables|/Script/Engine.Controller|GetPlayerState Instigater)))
  (Default|IncrementScore _asmy_player_state)
  (switch int (Variables|Default|Get掉落)
    (:1
      (Game|SpawnActorfromClass "/Game/blueprint/Buff.Buff_C" _returnvalue "Undefined" 0 0 :!label _label))
    (:2
      (Game|SpawnActorfromClass "/Game/blueprint/AKM.AKM_C" _returnvalue "Undefined" 0 false 0))
    (:3
      (goto _label))
    (:4
      (goto _label))))

(event Custom|SetHealthWight
  (bind _ashealth (Utilities|Casting|CastToHealth (UserInterface|GetWidget (Variables|Default|GetWidget))))
  (Variables|/Game/blueprint/widget/Health.Health_C|Sethealth _ashealth (Variables|Default|GetHealth)))

(event EventBeginPlay
  (bind _ashealth (Utilities|Casting|CastToHealth (UserInterface|GetWidget (Variables|Default|GetWidget))))
  (Variables|/Game/blueprint/widget/Health.Health_C|Setmaxhealth _ashealth (Variables|Default|GetMaxHealth))
  (Variables|/Game/blueprint/widget/Health.Health_C|Sethealth _ashealth (Variables|Default|GetHealth))
  (Variables|Default|Set掉落 (Math|Random|RandomInteger 7)))

(event Collision|EventActorBeginOverlap
  (params (OtherActor :type Actor%20Object%20Reference)))

(event Game|Damage|EventAnyDamage
  (params (Damage :type Float%20%28single-precision%29) (DamageType :type Damage%20Type%20Object%20Reference) (InstigatedBy :type Controller%20Object%20Reference) (DamageCauser :type Actor%20Object%20Reference))
  (Variables|Default|SetEnemy (Pawn|GetControlledPawn InstigatedBy))
  (if (<= (- (Variables|Default|Gethealth) Damage) 0.0)
    (Variables|Default|Sethealth 0.0)
    (CallFunction|Die InstigatedBy)
    (else
      (Variables|Default|Sethealth (- (Variables|Default|Gethealth) Damage))))
  (CallFunction|SetHealthWight))

(event EventTick
  (params (DeltaSeconds :type Float%20%28single-precision%29))
  (Transformation|SetWorldRotation (Variables|Default|GetWidget) (Math|Rotator|FindLookatRotation (Transformation|GetWorldLocation (Variables|Default|GetWidget)) (Camera|GetCameraLocation (Game|GetPlayerCameraManager 0))) false false))

(fn ConstructionScript)