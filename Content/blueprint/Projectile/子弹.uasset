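; Bullet projectile that flies as a physics sphere and turns into an explosion when it slows down.
; BeginPlay launches the Sphere along the actor's forward vector at Speed.
; Tick watches its velocity and, once it drops to a threshold, spawns an Explosion actor a single time, then destroys the bullet after a short delay.
; Hit is empty; the direct Enemy damage and particle logic is disconnected and never runs.
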(event EventBeginPlay
  (Physics|SetPhysicsLinearVelocity (Variables|Default|GetSphere) (* (Math|Vector|GetForwardVector (Transformation|GetActorRotation)) (Variables|Default|Getspeed)) false "None"))

(event Collision|EventActorBeginOverlap
  (params (OtherActor :type Actor%20Object%20Reference)))

(event EventTick
  (params (DeltaSeconds :type Float%20%28single-precision%29))
  (bind _returnvalue (Physics|GetPhysicsLinearVelocity (Variables|Default|GetSphere) "None"))
  (if (<= (Math|Vector|VectorLength _returnvalue) 5e+02)
    (Utilities|FlowControl|DoOnce false
      (:Completed
        (Game|SpawnActorfromClass "/Game/blueprint/Projectile/Explosion.Explosion_C" (Transformation|GetWorldTransform (Variables|Default|GetSphere)) "AlwaysSpawn" 0 0)
        (Utilities|FlowControl|Delay 0.2)
        (Actor|DestroyActor)))))

(event Collision|EventHit
  (params (MyComp :type Primitive%20Component%20Object%20Reference) (Other :type Actor%20Object%20Reference) (OtherComp :type Primitive%20Component%20Object%20Reference) (bSelfMoved :type Boolean) (HitLocation :type Vector :default "0, 0, 0") (HitNormal :type Vector :default "0, 0, 0") (NormalImpulse :type Vector :default "0, 0, 0") (Hit :type Hit%20Result%20Structure%20%28by%20ref%29)))

(fn ConstructionScript)