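; A player state Blueprint that holds a player's score, health and death count.
; Three functions modify these values: two increment score and deaths by one, and DecreaseHealth subtracts damage and returns the remaining health.
; Health is not clamped and no death check happens here, as the event graph and construction script are empty.
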(event EventBeginPlay)

(event EventTick
  (params (DeltaSeconds :type Float%20%28single-precision%29)))

(fn ConstructionScript)

(fn IncrementScore
  (Variables|Default|SetSc (+ (Variables|Default|GetSc) 1)))

(fn DecreaseHealth
  (params (Damage :type Float%20%28single-precision%29))
  (bind _output_get (Variables|Default|SetHealth (- (Variables|Default|GetHealth) Damage)))
  (return _output_get))

(fn IncrementDeath
  (Variables|Default|SetDeath (+ (Variables|Default|GetDeath) 1)))