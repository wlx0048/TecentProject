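; Bullet projectile actor that damages enemies on impact.
; On BeginPlay it launches its physics Sphere along the actor's forward vector at the Speed variable.
; On Hit it applies BaseDamage if the other actor is an Enemy, then destroys itself whatever it struck.
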(event EventBeginPlay
  (Physics|SetPhysicsLinearVelocity (Variables|Default|GetSphere) (* (Math|Vector|GetForwardVector (Transformation|GetActorRotation)) (Variables|Default|Getspeed)) false "None"))

(event Collision|EventActorBeginOverlap
  (params (OtherActor :type Actor%20Object%20Reference)))

(event EventTick
  (params (DeltaSeconds :type Float%20%28single-precision%29)))

(event Collision|EventHit
  (params (MyComp :type Primitive%20Component%20Object%20Reference) (Other :type Actor%20Object%20Reference) (OtherComp :type Primitive%20Component%20Object%20Reference) (bSelfMoved :type Boolean) (HitLocation :type Vector :default "0, 0, 0") (HitNormal :type Vector :default "0, 0, 0") (NormalImpulse :type Vector :default "0, 0, 0") (Hit :type Hit%20Result%20Structure%20%28by%20ref%29))
  (bind _asenemy (Utilities|Casting|CastToEnemy Other)
    (:then
      (Game|Damage|ApplyDamage _asenemy (Variables|Default|GetBase%20Damage) 0 0)
      (Actor|DestroyActor))
    (:CastFailed
      (Actor|DestroyActor))))

(fn ConstructionScript)