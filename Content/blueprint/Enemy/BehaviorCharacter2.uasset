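; Enemy character Blueprint for an armed AI that works with EnemyController_2.
; On BeginPlay it spawns an AKM, stores it as its weapon and attaches it to the mesh's gun socket.
; Taking damage records the damage causer and calls SetReceived on the controller.
; A SpawnProjectile event spawns a bullet (子弹) with fixed base damage at Arrow1's transform.
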(event Custom|SpawnProjectile
  (Game|SpawnActorfromClass "/Game/blueprint/Projectile/子弹.子弹_C" (Transformation|GetWorldTransform (Variables|Default|GetArrow1)) "AdjustIfPossibleButAlwaysSpawn" 0 1e+01 0))

(event Collision|EventActorBeginOverlap
  (params (OtherActor :type Actor%20Object%20Reference))
  (|CallParentFunction OtherActor) ; 此节点被禁用，将不会被调用。\n从引脚连出引线来编译功能。
)

(event EventTick
  (params (DeltaSeconds :type Float%20%28single-precision%29))
  (|CallParentFunction DeltaSeconds) ; 此节点被禁用，将不会被调用。\n从引脚连出引线来编译功能。
)

(event Game|Damage|EventAnyDamage
  (params (Damage :type Float%20%28single-precision%29) (DamageType :type Damage%20Type%20Object%20Reference) (InstigatedBy :type Controller%20Object%20Reference) (DamageCauser :type Actor%20Object%20Reference))
  (Variables|Default|SetDamage%20Causer DamageCauser)
  (bind _asenemy_controller_2 (Utilities|Casting|CastToEnemyController_2 (Pawn|GetController)))
  (Default|SetReceived _asenemy_controller_2))

(event EventBeginPlay
  (|CallParentFunction)
  (bind _returnvalue (Game|SpawnActorfromClass "/Game/blueprint/AKM.AKM_C" (Transformation|GetActorTransform self) "Undefined" 0 true 0))
  (Variables|Default|SetWeapon _returnvalue)
  (Transformation|AttachComponentToComponent (Variables|/Script/Engine.Actor|GetRootComponent _returnvalue) (Variables|Character|GetMesh) "gun" "SnapToTarget" "SnapToTarget" "KeepRelative" true))

(fn ConstructionScript
  (|CallParentFunction))