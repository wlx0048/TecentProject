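; A material study actor that randomizes its mesh's opacity while the player character (主角) is inside its sphere trigger.
; BeginPlay creates and stores a dynamic instance of M_Study_Inst on the static mesh.
; Sphere overlap starts a looping one-second timer that calls MaterialChange to set a random "不透明度" (opacity) scalar parameter.
; End overlap clears that timer by function name, leaving the last opacity in place.
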(event OnComponentBeginOverlap(Sphere)
  (params (OverlappedComponent :type Primitive%20Component%20Object%20Reference) (OtherActor :type Actor%20Object%20Reference) (OtherComp :type Primitive%20Component%20Object%20Reference) (OtherBodyIndex :type Integer) (bFromSweep :type Boolean) (SweepResult :type Hit%20Result%20Structure%20%28by%20ref%29))
  (Utilities|Casting|CastTo主角 OtherActor)
  (Utilities|Time|SetTimerbyEvent (delegate Custom|MaterialChange) 1.0 true))

(event OnComponentEndOverlap(Sphere)
  (params (OverlappedComponent :type Primitive%20Component%20Object%20Reference) (OtherActor :type Actor%20Object%20Reference) (OtherComp :type Primitive%20Component%20Object%20Reference) (OtherBodyIndex :type Integer))
  (Utilities|Casting|CastTo主角 OtherActor)
  (Utilities|Time|ClearTimerbyFunctionName 0 "MaterialChange"))

(event Custom|MaterialChange
  (Rendering|Material|SetScalarParameterValue (Variables|Default|GetMaterial) "不透明度" (Math|Random|RandomFloatinRange 0.0 1.0) :!class /Script/Engine.MaterialInstanceDynamic))

(event EventBeginPlay
  (bind _returnvalue (Rendering|Material|CreateDynamicMaterialInstance (Variables|Default|GetStaticMesh) 0 "/Game/Material/M_Study_Inst.M_Study_Inst" "None" :!class /Script/Engine.PrimitiveComponent))
  (Variables|Default|SetMaterial _returnvalue))

(event Collision|EventActorBeginOverlap
  (params (OtherActor :type Actor%20Object%20Reference)))

(event EventTick
  (params (DeltaSeconds :type Float%20%28single-precision%29)))

(fn ConstructionScript)