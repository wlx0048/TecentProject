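; Enemy character Blueprint that chases the ThirdPersonCharacter and deals contact damage while attacking.
; On BeginPlay it starts a looping AIMoveTo: each success raises CanAttack on the Boss_Animation instance for a few seconds, then resumes the chase; failed moves do not retry.
; A Box attached to the mesh applies damage when the player begins overlapping it, only while CanAttack is set.
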(event OnComponentBeginOverlap(Box)
  (params (OverlappedComponent :type Primitive%20Component%20Object%20Reference) (OtherActor :type Actor%20Object%20Reference) (OtherComp :type Primitive%20Component%20Object%20Reference) (OtherBodyIndex :type Integer) (bFromSweep :type Boolean) (SweepResult :type Hit%20Result%20Structure%20%28by%20ref%29))
  (bind _asthird_person_character (Utilities|Casting|CastToThirdPersonCharacter OtherActor))
  (bind _asboss_animation (Utilities|Casting|CastToBoss_Animation (Components|SkeletalMesh|GetAnimInstance (Variables|Character|GetMesh))))
  (if (Variables|/Game/BossyEnemy/Animations/InPlace/Movement/Boss_Animation.Boss_Animation_C|GetCan%20Attack _asboss_animation)
    (Game|Damage|ApplyDamage _asthird_person_character 1e+01 0 0)))

(event Custom|追踪
  (bind _returnvalue (Actor|GetActorOfClass "/Game/blueprint/ThirdPersonCharacter.ThirdPersonCharacter_C"))
  (AI|AIMoveTo self "0, 0, 0" _returnvalue 5.0 false :!label _label
    (:OnSuccess
      (bind _asboss_animation (Utilities|Casting|CastToBoss_Animation (Components|SkeletalMesh|GetAnimInstance (Variables|Character|GetMesh))))
      (Variables|/Game/BossyEnemy/Animations/InPlace/Movement/Boss_Animation.Boss_Animation_C|SetCan%20Attack _asboss_animation true)
      (Utilities|FlowControl|Delay 4.0)
      (Variables|/Game/BossyEnemy/Animations/InPlace/Movement/Boss_Animation.Boss_Animation_C|SetCan%20Attack _asboss_animation false)
      (goto _label))))

(event EventBeginPlay
  (|CallParentFunction)
  (CallFunction|追踪)
  (Transformation|AttachComponentToComponent (Variables|Default|GetBox) (Variables|Character|GetMesh) "None" "KeepRelative" "KeepRelative" "KeepRelative" true))

(event Collision|EventActorBeginOverlap
  (params (OtherActor :type Actor%20Object%20Reference)))

(fn ConstructionScript)