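; Boss enemy that charges in a straight line, attacking after each successful move.
; BeginPlay sets its health and computes a one-time look-at rotation toward the player character, which fixes the charge direction.
; A looping timer, gated by IsMove, issues AI moves along that direction; each success spawns BP_Fire and resets the gate after a delay.
; At half health or below, each success also spawns scaled-up Fog at a random nearby navigable point.
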(event Custom|Track
  (if (not (Variables|Default|GetisMove))
    (Variables|Default|SetisMove true)
    (AI|AIMoveTo self (+ (Transformation|GetActorLocation) (* (Math|Vector|GetForwardVector (Variables|Default|GetRotation)) 1e+03)) 0 5.0 false
      (:OnSuccess
        (CallFunction|攻击)
        (if (<= (Variables|Default|GetHealth) (/ (Variables|Default|GetMaxHealth) 2.0))
          (CallFunction|Crazy))
        (Utilities|FlowControl|Delay 1.0)
        (Variables|Default|SetisMove false)))))

(event Custom|攻击
  (Game|SpawnActorfromClass "/Game/blueprint/BP_Fire.BP_Fire_C" (Transformation|GetActorTransform) "Undefined" 0 0))

(event Custom|Crazy
  (bind _randomlocation (Class|NavigationSystemV1|GetRandomLocationinNavigableRadius (Transformation|GetActorLocation) 4e+02 0 0))
  (Game|SpawnActorfromClass "/Game/blueprint/Fog.Fog_C" (Math|Transform|MakeTransform _randomlocation "0, 0, 0" "3.750000,3.750000,3.750000") "Undefined" 0 0))

(event EventBeginPlay
  (|CallParentFunction)
  (Variables|Default|SetMaxHealth 5e+02)
  (Variables|Default|SetHealth 5e+02)
  (bind _returnvalue (Actor|GetActorOfClass "/Game/blueprint/ThirdPersonCharacter.ThirdPersonCharacter_C"))
  (bind _output_get (Variables|Default|SetRotation (Math|Rotator|FindLookatRotation (Transformation|GetActorLocation) (Transformation|GetActorLocation _returnvalue))))
  (Transformation|SetActorRotation _output_get)
  (Utilities|Time|SetTimerbyEvent (delegate Custom|Track) 0.1 true))

(event Collision|EventActorBeginOverlap
  (params (OtherActor :type Actor%20Object%20Reference))
  (|CallParentFunction OtherActor) ; 此节点被禁用，将不会被调用。\n从引脚连出引线来编译功能。
)

(event EventTick
  (params (DeltaSeconds :type Float%20%28single-precision%29))
  (|CallParentFunction DeltaSeconds))

(fn ConstructionScript
  (|CallParentFunction))