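; Multiplayer game mode that handles player spawning, match flow and a saved score leaderboard.
; PostLogin possesses a new character at successive PlayerStarts, while Respawn counts deaths and respawns at the first start after a delay.
; A GameState countdown triggers the spawn point and enemy spawners, which CometoEnd later replaces with a Boss.
; SaveList appends player zero's score to a save slot, and listshow bubble-sorts entries descending into scroll-box widgets.
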(event Custom|SaveList
  (bind _returnvalue (Game|GetPlayerController 0))
  (bind _playerstate (Variables|/Script/Engine.Controller|GetPlayerState _returnvalue))
  (bind _asmy_player_state (Utilities|Casting|CastToMyPlayerState _playerstate))
  ;[1 1 1] GameSave
  (bind _returnvalue_2 (SaveGame|DoesSaveGameExist "123"))
  (if _returnvalue_2
    (bind _returnvalue_3 (SaveGame|LoadGamefromSlot "123"))
    (bind _asmy_save_game (Utilities|Casting|CastToMySaveGame _returnvalue_3))
    (Variables|Default|SetGameSave _asmy_save_game)
    (else
      (bind _returnvalue_4 (SaveGame|CreateSaveGameObject "/Game/blueprint/rank/MySaveGame.MySaveGame_C"))
      (Variables|Default|SetGameSave _returnvalue_4)))
  (Utilities|Array|Add (Variables|/Game/blueprint/rank/MySaveGame.MySaveGame_C|GetSaveInfo (Variables|Default|GetGameSave)) (Utilities|Struct|Makerank (Variables|/Game/blueprint/myplayerstate.MyPlayerState_C|GetPlayerName _asmy_player_state) (Variables|/Game/blueprint/myplayerstate.MyPlayerState_C|GetSc _asmy_player_state)))
  (SaveGame|SaveGametoSlot (Variables|Default|GetGameSave) "123"))

(event Custom|Sort
  ;[1 1 1] listshow
  (CallFunction|List (Variables|/Game/blueprint/rank/MySaveGame.MySaveGame_C|GetSaveInfo (Variables|Default|GetGameSave))))

(event Custom|listshow
  ;[1 1 1] listshow
  (bind _returnvalue (SaveGame|LoadGamefromSlot "123"))
  (bind _asmy_save_game (Utilities|Casting|CastToMySaveGame _returnvalue))
  (Variables|Default|SetGameSave _asmy_save_game)
  (CallFunction|Sort)
  (bind _returnvalue_2 (UserInterface|CreateWidget "/Game/blueprint/rank/SaveHUD.SaveHUD_C"))
  (bind _output_get (Variables|Default|SetSaveHUD _returnvalue_2))
  (UserInterface|Viewport|AddtoViewport _output_get 0)
  (for _array_element (Variables|Default|GetSave)
    (bind _returnvalue_3 (UserInterface|CreateWidget "/Game/blueprint/rank/Onepiece.Onepiece_C" 0 (.CharacterName (Utilities|Struct|Breakrank _array_element)) (.Score (Utilities|Struct|Breakrank _array_element))))
    (Widget|Panel|AddChild (Variables|/Game/blueprint/rank/SaveHUD.SaveHUD_C|GetScrollBox_0 (Variables|Default|GetSaveHUD)) _returnvalue_3)))

(event Custom|CometoEnd
  (bind _outactors (Actor|GetAllActorsOfClass "/Game/blueprint/敌人刷新点.敌人刷新点_C"))
  (for _array_element _outactors
    (Actor|DestroyActor _array_element))
  (Game|SpawnActorfromClass "/Game/blueprint/Enemy/Boss.Boss_C" (Math|Transform|MakeTransform "-2490.000000,-210.000000,-2205.000000" "0,159.000000, 0") "Undefined" 0 0))

(event Custom|TimeDecrement
  (bind _asmy_game_state (Utilities|Casting|CastToMyGameState (Game|GetGameState)))
  (bind _newparam (Default|TimeDecrement _asmy_game_state))
  (if (<= _newparam 0.0)
    (Utilities|Time|ClearTimerbyFunctionName 0 "TimeDecrement")
    (bind _returnvalue (Actor|GetActorOfClass "/Game/blueprint/出生点.出生点_C"))
    (Default|Spawn _returnvalue)
    (bind _outactors (Actor|GetAllActorsOfClass "/Game/blueprint/敌人刷新点.敌人刷新点_C"))
    (for _array_element _outactors
      (Default|敌人刷新 _array_element))))

(event Custom|Respawn
  (params (Die :type Controller%20Object%20Reference))
  (bind _asmy_player_state (Utilities|Casting|CastToMyPlayerState (Variables|/Script/Engine.Controller|GetPlayerState Die)))
  (Default|IncrementDeath _asmy_player_state)
  (Utilities|FlowControl|Delay 3.0)
  (bind _outactors (Actor|GetAllActorsOfClass "/Script/Engine.PlayerStart"))
  (bind _returnvalue (Game|SpawnActorfromClass "/Game/blueprint/主角.主角_C" (Transformation|GetActorTransform (Utilities|Array|Get(acopy) _outactors)) "AdjustIfPossibleButAlwaysSpawn" 0 0))
  (Pawn|Possess Die _returnvalue)
  (bind _as1playercontroller (Utilities|Casting|CastTo1playercontroller Die))
  (Default|ResetHealth _as1playercontroller))

(event EventBeginPlay
  (Utilities|Time|SetTimerbyEvent (delegate Custom|TimeDecrement) 1.0 true))

(event EventPostLogin
  (params (NewPlayer :type Player%20Controller%20Object%20Reference))
  (bind _outactors (Actor|GetAllActorsOfClass "/Script/Engine.PlayerStart"))
  (bind _returnvalue (Game|SpawnActorfromClass "/Game/blueprint/主角.主角_C" (Transformation|GetActorTransform (Utilities|Array|Get(acopy) _outactors (Variables|Default|Getplayerindex))) "AdjustIfPossibleButAlwaysSpawn" 0 0))
  (Pawn|Possess NewPlayer _returnvalue)
  (Variables|Default|Setplayerindex (+ (Variables|Default|Getplayerindex) 1))
  (bind _asmy_player_state (Utilities|Casting|CastToMyPlayerState (Variables|/Script/Engine.Controller|GetPlayerState NewPlayer)))
  (Variables|/Game/blueprint/myplayerstate.MyPlayerState_C|SetPlayerNumber _asmy_player_state (Utilities|Array|Length (Variables|/Script/Engine.GameStateBase|GetPlayerArray (Game|GetGameState))))
  (bind _as1playercontroller (Utilities|Casting|CastTo1playercontroller NewPlayer))
  (Default|ClientLoginon _as1playercontroller))

(fn ConstructionScript)

(fn List
  (params (输入 :type Array%20of%20Rank%20Structures))
  (Variables|Default|SetSave 输入)
  (bind _output_get (LocalVariables|Setlength (Utilities|Array|Length (Variables|Default|GetSave))))
  (for _index (range 0 (- _output_get 1))
    (for _index_2 (range 0 (- (- (- _output_get 1) 1) _index))
      (if (<= (.Score (Utilities|Struct|Breakrank (Utilities|Array|Get(acopy) (Variables|Default|GetSave) _index_2))) (.Score (Utilities|Struct|Breakrank (Utilities|Array|Get(acopy) (Variables|Default|GetSave) (+ _index_2 1)))))
        (Utilities|Array|Swap (Variables|Default|GetSave) _index_2 (+ _index_2 1))))))