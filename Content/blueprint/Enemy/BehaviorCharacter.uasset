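; BehaviorCharacter is an enemy character Blueprint that reports incoming damage to its AI controller.
; On AnyDamage it stores the damage causer and calls SetReceived on its EnemyController, without changing any health value itself.
; UpdateWalkingSpeed exposes a setter for the movement component's max walk speed.
; BeginPlay, overlap and Tick are disabled stubs.
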(event EventBeginPlay
  (|CallParentFunction) ; 此节点被禁用，将不会被调用。\n从引脚连出引线来编译功能。
)

(event Collision|EventActorBeginOverlap
  (params (OtherActor :type Actor%20Object%20Reference))
  (|CallParentFunction OtherActor) ; 此节点被禁用，将不会被调用。\n从引脚连出引线来编译功能。
)

(event EventTick
  (params (DeltaSeconds :type Float%20%28single-precision%29))
  (|CallParentFunction DeltaSeconds) ; 此节点被禁用，将不会被调用。\n从引脚连出引线来编译功能。
)

(event Game|Damage|EventAnyDamage
  (params (Damage :type Float%20%28single-precision%29) (DamageType :type Damage%20Type%20Object%20Reference) (InstigatedBy :type Controller%20Object%20Reference) (DamageCauser :type Actor%20Object%20Reference))
  (Variables|Default|SetDamage%20Causer DamageCauser)
  (bind _asenemy_controller (Utilities|Casting|CastToEnemyController (Pawn|GetController)))
  (Default|SetReceived _asenemy_controller))

(fn ConstructionScript
  (|CallParentFunction))

(fn UpdateWalkingSpeed
  (params (NewSpeed :type Float%20%28single-precision%29))
  (Variables|/Script/Engine.CharacterMovementComponent|SetMaxWalkSpeed (Variables|Character|GetCharacterMovement) NewSpeed))